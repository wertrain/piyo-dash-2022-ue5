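; BP_World is the spherical world actor, scaled on construction to WORLDRADIUS() / 50.
; CreateObstacle converts spherical angles to a position, spawns a BP_Obstacle oriented away from a given center, and attaches it to the world.
; CreateObstacles repeats this with random angles, while a deprecated variant builds an evenly spaced ring.
; Event graph events are empty; its obstacle spawning and rotation tests are disconnected and never run.
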(event EventBeginPlay)

(event Collision|EventActorBeginOverlap
  (params (OtherActor :type Actor%20Object%20Reference)))

(event EventTick
  (params (DeltaSeconds :type Float%20%28single-precision%29)))

(fn ConstructionScript
  (bind _world_radius (Utilities|WORLDRADIUS))
  (bind _returnvalue (/ _world_radius 5e+01))
  (Transformation|SetWorldScale3D (Variables|Default|GetDefaultSceneRoot) (Math|Vector|MakeVector _returnvalue _returnvalue _returnvalue)))

(fn DeprecatedCreateObstacles
  (params (In%20Number :type Integer) (In%20Center :type Vector) (In%20Radius :type Float%20%28double-precision%29))
  (LocalVariables|SetDegree%20Interval (/ 3.6e+02 (Math|Conversions|ToFloat(Integer) In%20Number)))
  (for _index (range 0 In%20Number)
    (Game|SpawnActorfromClass "/Game/PiyoDash/Core/Characters/BP_Obstacle.BP_Obstacle_C" (Math|Transform|MakeTransform (+ (Math|Vector|MakeVector 0.0 (* (Math|Trig|Cos(Degrees) (* (LocalVariables|GetDegree%20Interval) (Math|Conversions|ToFloat(Integer) _index))) In%20Radius) (* (Math|Trig|Sin(Degrees) (* (LocalVariables|GetDegree%20Interval) (Math|Conversions|ToFloat(Integer) _index))) In%20Radius)) In%20Center) (Math|Rotator|MakeRotator (* (+ (* (LocalVariables|GetDegree%20Interval) (Math|Conversions|ToFloat(Integer) _index)) 9e+01) -1.0) 0.0 0.0)) "Undefined" self 0)))

(fn CreateObstacle
  (params (In%20Radius :type Float%20%28double-precision%29) (In%20Theta :type Float%20%28double-precision%29) (In%20Phai :type Float%20%28double-precision%29) (In%20Center :type Vector))
  (bind _output_get (LocalVariables|SetPosition (Math|Vector|MakeVector (* (Math|Trig|Sin(Degrees) In%20Theta) (Math|Trig|Cos(Degrees) In%20Phai) In%20Radius) (* (Math|Trig|Sin(Degrees) In%20Theta) (Math|Trig|Sin(Degrees) In%20Phai) In%20Radius) (* (Math|Trig|Cos(Degrees) In%20Theta) In%20Radius))))
  (bind _returnvalue (Game|SpawnActorfromClass "/Game/PiyoDash/Core/Characters/BP_Obstacle.BP_Obstacle_C" (Math|Transform|MakeTransform _output_get (Math|Rotator|MakeRotator (.Roll (Math|Rotator|BreakRotator (Class|KismetMathLibrary|QuatRotator (Math|Conversions|ToQuaternion(Rotator) (- (LocalVariables|GetPosition) In%20Center))))) (+ (.Pitch (Math|Rotator|BreakRotator (Class|KismetMathLibrary|QuatRotator (Math|Conversions|ToQuaternion(Rotator) (- (LocalVariables|GetPosition) In%20Center))))) 9e+01) (.Yaw (Math|Rotator|BreakRotator (Class|KismetMathLibrary|QuatRotator (Math|Conversions|ToQuaternion(Rotator) (- (LocalVariables|GetPosition) In%20Center))))))) "Undefined" self 0))
  (Transformation|AttachActorToActor _returnvalue self "None" "KeepRelative" "KeepRelative" "KeepRelative" true))

(fn CreateObstacles
  (params (In%20Number :type Integer) (In%20Center :type Vector) (In%20Radius :type Float%20%28double-precision%29))
  (for _index (range 0 In%20Number)
    (CallFunction|CreateObstacle In%20Radius (* (Math|Random|RandomFloat) 3.6e+02) (* (Math|Random|RandomFloat) 3.6e+02) In%20Center)))