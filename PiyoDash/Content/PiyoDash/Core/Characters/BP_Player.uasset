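; Player character for PiyoDash that moves on a spherical world, its transform built each Tick from one quaternion plus a height.
; Input flags rotate the quaternion to turn or advance; advancing requires a downward trace ahead to hit, which sets ground height.
; Jumps use manual force and gravity, with an explosion effect on press.
; Attack spawns BP_Bomb, capped at three live bombs via their destroy callback.
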(event Custom|OnDestroyed_Bomb
  (params (DestroyedActor :type Actor%20Object%20Reference))
  (Math|Integer|DecrementInt (Variables|Default|GetBombCount)))

(event EventBeginPlay)

(event Collision|EventActorBeginOverlap
  (params (OtherActor :type Actor%20Object%20Reference)))

(event EventTick
  (params (DeltaSeconds :type Float%20%28single-precision%29))
  (Utilities|FlowControl|Sequence
    (:then_0
      ;[1 1 1] 一つのクオータニオンと高さのみで、位置と向きを表現する： https://dixq.net/forum/viewtopic.php?t=13625
      (Transformation|SetWorldTransform (Variables|Default|GetScene) (Math|Transform|MakeTransform (Class|KismetMathLibrary|QuatRotateVector (Variables|Default|GetQuat) (Math|Vector|MakeVector 0.0 0.0 (+ (Variables|Default|GetPositionZ) (Utilities|WORLDRADIUS)))) (Class|KismetMathLibrary|QuatRotator (Variables|Default|GetQuat))) false false)
      (Development|PrintText (Utilities|Text|FormatText "{0} {1} {2} {3}" (.X (Class|KismetMathLibrary|BreakQuat (Variables|Default|GetQuat))) (.Y (Class|KismetMathLibrary|BreakQuat (Variables|Default|GetQuat))) (.Z (Class|KismetMathLibrary|BreakQuat (Variables|Default|GetQuat))) (.W (Class|KismetMathLibrary|BreakQuat (Variables|Default|GetQuat)))) true true "(R=0.000000,G=0.660000,B=1.000000,A=1.000000)" 0.0))
    (:then_1
      (if (Variables|Default|GetbIsPressLeft)
        ;[1 1 1] 左方向への回転
        (Variables|Default|SetQuat (* (Math|Vector|RotatorfromAxisandAngle (Class|KismetMathLibrary|QuatVectorUp (Variables|Default|GetQuat)) (* (Utilities|RotateSpeed) -1.0)) (Variables|Default|GetQuat)))))
    (:then_2
      (if (Variables|Default|GetbIsPressRight)
        ;[1 1 1] 右方向への回転
        (Variables|Default|SetQuat (* (Math|Vector|RotatorfromAxisandAngle (Class|KismetMathLibrary|QuatVectorUp (Variables|Default|GetQuat)) (Utilities|RotateSpeed)) (Variables|Default|GetQuat)))))
    (:then_3
      (if (Variables|Default|GetbIsPressForward)
        ;[1 1 1] 正面方向への移動
        (bind (_out_is_hit _out_ground_positionz) (CallFunction|RaycatPlayerFront 5e+01 (Utilities|RaycastHeight)))
        (if _out_is_hit
          (Variables|Default|SetGroundPositionZ _out_ground_positionz)
          (Variables|Default|SetQuat (* (Math|Vector|RotatorfromAxisandAngle (Math|Vector|CrossProduct (Class|KismetMathLibrary|QuatVectorUp (Variables|Default|GetQuat)) (Class|KismetMathLibrary|QuatVectorForward (Variables|Default|GetQuat))) (Utilities|ForwardSpeed)) (Variables|Default|GetQuat))))))
    (:then_4
      (if (Variables|Default|GetbIsPressJump)
        ;[1 1 1] ジャンプ処理
        (if (not (Variables|Default|GetbIsJumping))
          (Variables|Default|SetJumpForce (Utilities|JumpPower))
          (Variables|Default|SetbIsJumping true))))
    (:then_5
      (if (Variables|Default|GetbIsPressAttack)
        (if (< (Variables|Default|GetBombCount) 3)
          (bind _returnvalue (Game|SpawnActorfromClass "/Game/PiyoDash/Core/Characters/BP_Bomb.BP_Bomb_C" (Transformation|GetActorTransform) "Undefined" 0 0))
          (if (Utilities|IsValid _returnvalue)
            (Game|AssignOnDestroyed _returnvalue (delegate Custom|OnDestroyed_Bomb))
            (Math|Integer|IncrementInt (Variables|Default|GetBombCount)
              (:%20%20
                (Variables|Default|SetbIsPressAttack false)))))))
    (:then_7
      (Utilities|FlowControl|Sequence
        (:then_0
          ;[1 1 1] 重力
          (bind _output_get (Variables|Default|SetPositionZ (+ (Variables|Default|GetPositionZ) (Variables|Default|GetJumpForce))))
          (if (<= _output_get (Variables|Default|GetGroundPositionZ))
            (Variables|Default|SetbIsJumping false)
            (Variables|Default|SetPositionZ (Variables|Default|GetGroundPositionZ))
            (Variables|Default|SetJumpForce 0.0)))
        (:then_1
          (if (> (Variables|Default|GetPositionZ) (Variables|Default|GetGroundPositionZ))
            (bind _output_get_2 (Variables|Default|SetPositionZ (- (Variables|Default|GetPositionZ) (* (Utilities|WORLDGRAVITY) (Utilities|Time|GetWorldDeltaSeconds)))))
            (if (<= _output_get_2 (Variables|Default|GetGroundPositionZ))
              (Variables|Default|SetbIsJumping false)
              (Variables|Default|SetPositionZ (Variables|Default|GetGroundPositionZ))
              (Variables|Default|SetJumpForce 0.0))))
        (:then_2
          (if (Variables|Default|GetbIsJumping)
            (Variables|Default|SetJumpForce (- (Variables|Default|GetJumpForce) (* (Utilities|WORLDGRAVITY) (Utilities|Time|GetWorldDeltaSeconds))))
            (else
              (Variables|Default|SetPositionZ (Variables|Default|GetGroundPositionZ)))))))))

(event Input|ActionEvents|InputActionButtonRight
  (params (Key :type Key%20Structure :default "None"))
  (:Pressed
    (Variables|Default|SetbIsPressAttack true))
  (:Released
    (Variables|Default|SetbIsPressAttack false)))

(event Input|ActionEvents|InputActionCursorLeft
  (params (Key :type Key%20Structure :default "None"))
  (:Pressed
    (Variables|Default|SetbIsPressLeft true))
  (:Released
    (Variables|Default|SetbIsPressLeft false)))

(event Input|ActionEvents|InputActionCursorRight
  (params (Key :type Key%20Structure :default "None"))
  (:Pressed
    (Variables|Default|SetbIsPressRight true))
  (:Released
    (Variables|Default|SetbIsPressRight false)))

(event Input|ActionEvents|InputActionCursorUp
  (params (Key :type Key%20Structure :default "None"))
  (:Pressed
    (Variables|Default|SetbIsPressForward true))
  (:Released
    (Variables|Default|SetbIsPressForward false)))

(event Input|ActionEvents|InputActionButtonBottom
  (params (Key :type Key%20Structure :default "None"))
  (:Pressed
    (Variables|Default|SetbIsPressJump true)
    (Niagara|SpawnSystematLocation "/Game/PiyoDash/Effects/FXS_Explosion.FXS_Explosion" (Transformation|GetActorLocation)))
  (:Released
    (Variables|Default|SetbIsPressJump false)))

(fn ConstructionScript)

(fn RaycatPlayerFront
  (params (In%20Front%20Distance :type Float%20%28double-precision%29) (In%20Raycast%20Height :type Float%20%28double-precision%29))
  (bind _quat (Variables|Default|GetQuat))
  (bind _scene (Variables|Default|GetScene))
  (bind _quat_2 (Variables|Default|GetQuat))
  (bind _returnvalue (Transformation|GetWorldLocation _scene))
  (bind _returnvalue_2 (Class|KismetMathLibrary|QuatVectorForward _quat_2))
  (bind _returnvalue_3 (Class|KismetMathLibrary|QuatVectorUp _quat))
  (bind _returnvalue_4 (* _returnvalue_3 In%20Raycast%20Height))
  (bind _returnvalue_5 (* _returnvalue_2 In%20Front%20Distance))
  (bind _returnvalue_6 (+ _returnvalue _returnvalue_5 _returnvalue_4))
  (bind _outhit (Collision|LineTraceForObjects _returnvalue_6 (+ _returnvalue_6 (* (Math|Vector|NegateVector (Class|KismetMathLibrary|QuatVectorUp (Variables|Default|GetQuat))) (* In%20Raycast%20Height 2e+01))) (Utilities|Array|MakeArray "ObjectTypeQuery1") false 0 "ForDuration"))
  ;[1 1 1] 内積による壁判定
  (Development|PrintText (Utilities|Text|FormatText "{0}" (Math|Vector|DotProduct (.normal _outhit) (Class|KismetMathLibrary|QuatVectorUp (Variables|Default|GetQuat)))) true true "(R=0.000000,G=0.660000,B=1.000000,A=1.000000)" 0.0)
  (if (Math|Boolean|ANDBoolean (.bblockinghit _outhit) true true)
    (return true (- (Math|Vector|VectorLength (.location _outhit)) (Utilities|WORLDRADIUS)))
    (else
      (return false 0.0))))