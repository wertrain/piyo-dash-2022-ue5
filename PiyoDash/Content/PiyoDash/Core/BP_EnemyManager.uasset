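; Enemy manager for PiyoDash that spawns a BP_Enemy whenever a timer passes SpawnIntervalSec and prints the live array count each tick.
; SpawnEnemies creates enemies at the origin, stores them in Enemies, sets their Quat and binds their destroy event.
; GetRandomQuatPlayerAround holds only unused nodes for randomizing around the player ship's Quat.
; The destroy handler only casts; array removal and nearby-enemy chain destruction are disconnected.
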(event Custom|OnDestroyed_Enemy
  (params (DestroyedActor :type Actor%20Object%20Reference))
  (bind _asbp_enemy (Utilities|Casting|CastToBP_Enemy DestroyedActor)))

(event EventBeginPlay
  (bind _asbp_spaceship (Utilities|Casting|CastToBP_Spaceship (Game|Player|GetPlayerPawn 0)))
  (Variables|Default|SetPlayerPawn _asbp_spaceship))

(event Collision|EventActorBeginOverlap
  (params (OtherActor :type Actor%20Object%20Reference)))

(event EventTick
  (params (DeltaSeconds :type Float%20%28single-precision%29))
  (Utilities|FlowControl|Sequence
    (:then_0
      (bind _output_get (Variables|Default|SetSpawnTimer (+ DeltaSeconds (Variables|Default|GetSpawnTimer))))
      (if (> _output_get (Variables|Default|GetSpawnIntervalSec))
        (Variables|Default|SetSpawnTimer 0.0)
        (CallFunction|SpawnEnemies 0)))
    (:then_1
      (Development|PrintText (Utilities|Text|FormatText "Spawned Enemies {0}" (Utilities|Array|Length (Variables|Default|GetEnemies))) true true "(R=0.000000,G=0.660000,B=1.000000,A=1.000000)" 0.0))))

(fn ConstructionScript)

(fn SpawnEnemies
  (params (Count :type Integer))
  (for _index (range 1 (- Count -1))
    (bind _returnvalue (Game|SpawnActorfromClass "/Game/PiyoDash/Core/Characters/BP_Enemy.BP_Enemy_C" (Math|Transform|MakeTransform "0, 0, 0") "Undefined" 0 0))
    (LocalVariables|SetSpawned _returnvalue)
    (Utilities|Array|Add (Variables|Default|GetEnemies) (LocalVariables|GetSpawned))
    (Variables|/Game/PiyoDash/Core/Characters/BP_Enemy.BP_Enemy_C|SetQuat (LocalVariables|GetSpawned) (Utilities|GetRandomQuatPlayerAround))
    (Game|BindEventtoOnDestroyed (LocalVariables|GetSpawned) (EventDispatchers|CreateEvent :!event Custom|OnDestroyed_Enemy))))