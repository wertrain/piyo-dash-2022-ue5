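; BP_NormalProjectile is a short-lived projectile that travels around a spherical world and destroys Enemy-tagged actors overlapping its Box.
; Its position is stored as a quaternion, which GoForward rotates each Tick about the cross product of its up and forward vectors.
; UpdateTransformFromQuat converts that into world location and rotation, using world radius plus a height offset.
; A timer started at BeginPlay destroys the projectile when its lifetime ends.
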(event OnComponentBeginOverlap(Box)
  (params (OverlappedComponent :type Primitive%20Component%20Object%20Reference) (OtherActor :type Actor%20Object%20Reference) (OtherComp :type Primitive%20Component%20Object%20Reference) (OtherBodyIndex :type Integer) (bFromSweep :type Boolean) (SweepResult :type Hit%20Result%20Structure%20%28by%20ref%29))
  (if (Actor|ActorHasTag OtherActor "Enemy")
    (Actor|DestroyActor OtherActor)))

(event Custom|OnEndLifeTime
  (Actor|DestroyActor))

(event EventBeginPlay
  (CallFunction|UpdateTransformfromQuat)
  (Utilities|Time|SetTimerbyEvent (delegate Custom|OnEndLifeTime) 1.0))

(event Collision|EventActorBeginOverlap
  (params (OtherActor :type Actor%20Object%20Reference)))

(event EventTick
  (params (DeltaSeconds :type Float%20%28single-precision%29))
  (Utilities|FlowControl|Sequence
    (:then_0
      (CallFunction|GoForward (Utilities|ForwardSpeed))
      (CallFunction|UpdateTransformfromQuat))))

(fn ConstructionScript)

(fn UpdateTransformfromQuat
  (Transformation|SetWorldTransform (Variables|Default|GetDefaultSceneRoot) (Math|Transform|MakeTransform (Class|KismetMathLibrary|QuatRotateVector (Variables|Default|GetQuat) (Math|Vector|MakeVector 0.0 0.0 (+ (Variables|デフォルト|GetPositionZ) (Utilities|WORLDRADIUS)))) (Class|KismetMathLibrary|QuatRotator (Variables|Default|GetQuat))) false false))

(fn GoForward
  (params (In%20Speed :type Float%20%28double-precision%29))
  (Variables|Default|SetQuat (* (Math|Vector|RotatorfromAxisandAngle (Math|Vector|CrossProduct (Class|KismetMathLibrary|QuatVectorUp (Variables|Default|GetQuat)) (Class|KismetMathLibrary|QuatVectorForward (Variables|Default|GetQuat))) In%20Speed) (Variables|Default|GetQuat))))