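; Enemy actor that chases the BP_Player pawn across the surface of a spherical world, starting at a random spot.
; A single Quat encodes both position and heading; the transform is that rotation applied to world radius plus PositionZ.
; Each Tick snaps heading to the player via atan2 in local space, updates the transform, then rotates Quat forward by ForwardSpeed.
; RotateToPlayer and many disconnected nodes are unused earlier experiments.
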(event EventBeginPlay
  (bind _asbp_player (Utilities|Casting|CastToBP_Player (Game|Player|GetPlayerPawn 0)))
  (Variables|Default|SetPlayerPawn _asbp_player)
  ;[1 1 1] 初期はランダム位置に配置
  (Variables|Default|SetQuat (Math|Conversions|ToQuaternion(Rotator) (Math|Random|RandomRotator false))))

(event Collision|EventActorBeginOverlap
  (params (OtherActor :type Actor%20Object%20Reference)))

(event EventTick
  (params (DeltaSeconds :type Float%20%28single-precision%29))
  (Utilities|FlowControl|Sequence
    (:then_1
      (bind _angle (CallFunction|GetRelativePlayerDegree))
      (CallFunction|AddAngletoQuat _angle))
    (:then_3
      (CallFunction|UpdateTransformfromQuat))
    (:then_5
      (CallFunction|GoForward (Utilities|ForwardSpeed)))))

(fn ConstructionScript)

(fn GetRelativePlayerDegree
  (bind _playerpawn (Variables|Default|GetPlayerPawn))
  (bind _quat (Variables|Default|GetQuat))
  (bind _defaultsceneroot (Variables|Default|GetDefaultSceneRoot))
  (bind _returnvalue (Transformation|GetWorldLocation _defaultsceneroot))
  (bind _scene (Variables|/Game/PiyoDash/Core/Characters/BP_Player.BP_Player_C|GetScene _playerpawn))
  (bind _returnvalue_2 (Transformation|GetWorldLocation _scene))
  (bind _returnvalue_3 (- _returnvalue_2 _returnvalue))
  (bind _returnvalue_4 (Class|KismetMathLibrary|QuatUnrotateVector _quat _returnvalue_3))
  (bind (_x _y) (Math|Vector|BreakVector _returnvalue_4))
  (return (Class|KismetMathLibrary|DegAtan2 _y _x)))

(fn AddAngletoQuat
  (params (In%20Angle :type Float%20%28double-precision%29))
  (Variables|Default|SetQuat (* (Math|Vector|RotatorfromAxisandAngle (Class|KismetMathLibrary|QuatVectorUp (Variables|Default|GetQuat)) In%20Angle) (Variables|Default|GetQuat))))

(fn UpdateTransformfromQuat
  (Transformation|SetWorldTransform (Variables|Default|GetDefaultSceneRoot) (Math|Transform|MakeTransform (Class|KismetMathLibrary|QuatRotateVector (Variables|Default|GetQuat) (Math|Vector|MakeVector 0.0 0.0 (+ (Variables|Default|GetPositionZ) (Utilities|WORLDRADIUS)))) (Class|KismetMathLibrary|QuatRotator (Variables|Default|GetQuat))) false false))

(fn GoForward
  (params (In%20Speed :type Float%20%28double-precision%29))
  (Variables|Default|SetQuat (* (Math|Vector|RotatorfromAxisandAngle (Math|Vector|CrossProduct (Class|KismetMathLibrary|QuatVectorUp (Variables|Default|GetQuat)) (Class|KismetMathLibrary|QuatVectorForward (Variables|Default|GetQuat))) In%20Speed) (Variables|Default|GetQuat))))