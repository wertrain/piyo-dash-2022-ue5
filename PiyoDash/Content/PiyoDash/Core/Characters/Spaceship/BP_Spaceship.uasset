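; Player spaceship for PiyoDash that flies at fixed height around a spherical world and pauses the game when damaged.
; A single quaternion encodes position and heading; Tick rotates it for steering and constant forward motion, then derives the transform.
; Input flags adjust speed, bank the mesh with eased roll, and fire BP_NormalProjectile along that quaternion, capped at ten live shots.
; Jump, gravity, ground-trace and explosion logic is left unconnected.
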(event Custom|OnDestroyed_Bomb
  (params (DestroyedActor :type Actor%20Object%20Reference))
  (Math|Integer|DecrementInt (Variables|Default|GetShotCount)))

(event EventBeginPlay
  (Variables|Default|SetSpeed (Utilities|MinForwardSpeed)))

(event Collision|EventActorBeginOverlap
  (params (OtherActor :type Actor%20Object%20Reference)))

(event EventTick
  (params (DeltaSeconds :type Float%20%28single-precision%29))
  (Utilities|FlowControl|Sequence
    (:then_0
      (Variables|Default|SetRoll (Math|Float|Lerp (Variables|Default|GetRoll) 0.0 (Variables|Default|GetAttitudeTimer)))
      (bind _output_get (Variables|Default|SetAttitudeTimer (+ (* 0.3 (Utilities|GetCurrentSpeedRate) (Utilities|Time|GetWorldDeltaSeconds)) (Variables|Default|GetAttitudeTimer))))
      (if (> _output_get 1.0)
        (Variables|Default|SetAttitudeTimer 1.0)))
    (:then_1
      ;[1 1 1] 一つのクオータニオンと高さのみで、位置と向きを表現する： https://dixq.net/forum/viewtopic.php?t=13625
      (Transformation|SetWorldTransform (Variables|Default|GetScene) (Math|Transform|MakeTransform (Class|KismetMathLibrary|QuatRotateVector (Variables|Default|GetQuat) (Math|Vector|MakeVector 0.0 0.0 (+ 2e+02 (Utilities|WORLDRADIUS)))) (Class|KismetMathLibrary|QuatRotator (Variables|Default|GetQuat))) false false)
      (Development|PrintText (Utilities|Text|FormatText "{0} {1} {2} {3}" (.X (Class|KismetMathLibrary|BreakQuat (Variables|Default|GetQuat))) (.Y (Class|KismetMathLibrary|BreakQuat (Variables|Default|GetQuat))) (.Z (Class|KismetMathLibrary|BreakQuat (Variables|Default|GetQuat))) (.W (Class|KismetMathLibrary|BreakQuat (Variables|Default|GetQuat)))) true true "(R=0.000000,G=0.660000,B=1.000000,A=1.000000)" 0.0))
    (:then_2
      (if (Variables|Default|GetbIsPressLeft)
        ;[1 1 1] 左方向への回転
        (Variables|Default|SetQuat (* (Math|Vector|RotatorfromAxisandAngle (Class|KismetMathLibrary|QuatVectorUp (Variables|Default|GetQuat)) (* (Utilities|RotateSpeed) -1.0)) (Variables|Default|GetQuat)))
        (Variables|Default|SetAttitudeTimer 0.0)
        (bind _output_get_2 (Variables|Default|SetRoll (+ (Variables|Default|GetRoll) (* 0.015 (Utilities|GetCurrentSpeedRate)))))
        (if (> _output_get_2 0.8)
          (Variables|Default|SetRoll 0.8))))
    (:then_3
      (if (Variables|Default|GetbIsPressRight)
        ;[1 1 1] 右方向への回転
        (Variables|Default|SetQuat (* (Math|Vector|RotatorfromAxisandAngle (Class|KismetMathLibrary|QuatVectorUp (Variables|Default|GetQuat)) (Utilities|RotateSpeed)) (Variables|Default|GetQuat)))
        (Variables|Default|SetAttitudeTimer 0.0)
        (bind _output_get_3 (Variables|Default|SetRoll (- (Variables|Default|GetRoll) (* 0.015 (Utilities|GetCurrentSpeedRate)))))
        (if (<= _output_get_3 -0.8)
          (Variables|Default|SetRoll -0.8))))
    (:then_4
      (if (Variables|Default|GetbIsPressForward)
        (bind _output_get_4 (Variables|Default|SetSpeed (+ (Variables|Default|GetSpeed) (* (Utilities|Time|GetWorldDeltaSeconds) 0.1))))
        (if (> _output_get_4 (Utilities|MaxForwardSpeed))
          (Variables|Default|SetSpeed (Utilities|MaxForwardSpeed)))))
    (:then_5
      (if (Variables|Default|GetbIsPressBackward)
        (bind _output_get_5 (Variables|Default|SetSpeed (- (Variables|Default|GetSpeed) (* (Utilities|Time|GetWorldDeltaSeconds) 0.2))))
        (if (< _output_get_5 (Utilities|MinForwardSpeed))
          (Variables|Default|SetSpeed (Utilities|MinForwardSpeed)))))
    (:then_6
      ;[1 1 1] 正面方向への移動
      (Variables|Default|SetQuat (* (Math|Vector|RotatorfromAxisandAngle (Math|Vector|CrossProduct (Class|KismetMathLibrary|QuatVectorUp (Variables|Default|GetQuat)) (Class|KismetMathLibrary|QuatVectorForward (Variables|Default|GetQuat))) (Variables|Default|GetSpeed)) (Variables|Default|GetQuat))))
    (:then_7
      (if (Variables|Default|GetbIsPressAttack)
        (if (< (Variables|Default|GetShotCount) 10)
          (bind _returnvalue (Game|SpawnActorfromClass "/Game/PiyoDash/Core/Weapons/BP_NormalProjectile.BP_NormalProjectile_C" (Transformation|GetActorTransform) "Undefined" 0 0))
          (if (Utilities|IsValid _returnvalue)
            (Variables|/Game/PiyoDash/Core/Weapons/BP_NormalProjectile.BP_NormalProjectile_C|SetQuat _returnvalue (Variables|Default|GetQuat))
            (Game|AssignOnDestroyed _returnvalue (delegate Custom|OnDestroyed_Bomb))
            (Math|Integer|IncrementInt (Variables|Default|GetShotCount)
              (:%20%20
                (Variables|Default|SetbIsPressAttack false)))))))
    (:then_8
      (bind _out_value (CallFunction|GetSignValue (Variables|Default|GetRoll)))
      (Transformation|SetRelativeRotation (Variables|Default|GetStaticMesh) (Class|KismetMathLibrary|QuatRotator (* (Math|Conversions|ToQuaternion(Rotator) (Math|Vector|RotatorfromAxisandAngle "1.000000,0.000000,0.000000" (* _out_value (* (Math|Float|Absolute(Float) (Variables|Default|GetRoll)) 9e+01)))) (Math|Conversions|ToQuaternion(Rotator) (Math|Vector|RotatorfromAxisandAngle "0, 0,1.000000" -9e+01)))) false false))
    (:then_9)))

(event Game|Damage|EventAnyDamage
  (params (Damage :type Float%20%28single-precision%29) (DamageType :type Damage%20Type%20Object%20Reference) (InstigatedBy :type Controller%20Object%20Reference) (DamageCauser :type Actor%20Object%20Reference))
  (Development|PrintText "Damage")
  (Game|SetGamePaused true))

(event Input|ActionEvents|InputActionButtonRight
  (params (Key :type Key%20Structure :default "None"))
  (:Pressed
    (Variables|Default|SetbIsPressAttack true))
  (:Released
    (Variables|Default|SetbIsPressAttack false)))

(event Input|ActionEvents|InputActionCursorBottom
  (params (Key :type Key%20Structure :default "None"))
  (:Pressed
    (Variables|Default|SetbIsPressBackward true))
  (:Released
    (Variables|Default|SetbIsPressBackward false)))

(event Input|ActionEvents|InputActionCursorLeft
  (params (Key :type Key%20Structure :default "None"))
  (:Pressed
    (Variables|Default|SetbIsPressLeft true))
  (:Released
    (Variables|Default|SetbIsPressLeft false)))

(event Input|ActionEvents|InputActionCursorRight
  (params (Key :type Key%20Structure :default "None"))
  (:Pressed
    (Variables|Default|SetbIsPressRight true))
  (:Released
    (Variables|Default|SetbIsPressRight false)))

(event Input|ActionEvents|InputActionCursorUp
  (params (Key :type Key%20Structure :default "None"))
  (:Pressed
    (Variables|Default|SetbIsPressForward true))
  (:Released
    (Variables|Default|SetbIsPressForward false)))

(event Input|ActionEvents|InputActionButtonBottom
  (params (Key :type Key%20Structure :default "None"))
  (:Pressed
    (Variables|Default|SetbIsPressJump true))
  (:Released
    (Variables|Default|SetbIsPressJump false)))

(fn ConstructionScript)

(fn RaycatPlayerFront
  (params (In%20Front%20Distance :type Float%20%28double-precision%29) (In%20Raycast%20Height :type Float%20%28double-precision%29))
  (bind _quat (Variables|Default|GetQuat))
  (bind _scene (Variables|Default|GetScene))
  (bind _quat_2 (Variables|Default|GetQuat))
  (bind _returnvalue (Transformation|GetWorldLocation _scene))
  (bind _returnvalue_2 (Class|KismetMathLibrary|QuatVectorForward _quat_2))
  (bind _returnvalue_3 (Class|KismetMathLibrary|QuatVectorUp _quat))
  (bind _returnvalue_4 (* _returnvalue_3 In%20Raycast%20Height))
  (bind _returnvalue_5 (* _returnvalue_2 In%20Front%20Distance))
  (bind _returnvalue_6 (+ _returnvalue _returnvalue_5 _returnvalue_4))
  (bind _outhit (Collision|LineTraceForObjects _returnvalue_6 (+ _returnvalue_6 (* (Math|Vector|NegateVector (Class|KismetMathLibrary|QuatVectorUp (Variables|Default|GetQuat))) (* In%20Raycast%20Height 2e+01))) (Utilities|Array|MakeArray "ObjectTypeQuery1") false 0 "ForDuration"))
  ;[1 1 1] 内積による壁判定
  (Development|PrintText (Utilities|Text|FormatText "{0}" (Math|Vector|DotProduct (.normal _outhit) (Class|KismetMathLibrary|QuatVectorUp (Variables|Default|GetQuat)))) true true "(R=0.000000,G=0.660000,B=1.000000,A=1.000000)" 0.0)
  (if (Math|Boolean|ANDBoolean (.bblockinghit _outhit) true true)
    (return true (- (Math|Vector|VectorLength (.location _outhit)) (Utilities|WORLDRADIUS)))
    (else
      (return false 0.0))))

(fn GetSignValue
  (params (In%20Value :type Float%20%28double-precision%29))
  (if (>= In%20Value 0.0)
    (return 1.0)
    (else
      (return -1.0))))