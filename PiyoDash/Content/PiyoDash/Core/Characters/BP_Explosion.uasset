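; BP_Explosion is a short-lived blast actor that destroys enemies caught in its expanding sphere.
; The Sphere component starts at zero scale, grows linearly each Tick using delta time, and the actor destroys itself at maximum scale.
; When the sphere overlaps an actor tagged Enemy, it destroys that actor and spawns the FXS_Explosion Niagara effect at the blast's own location.
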(event OnComponentBeginOverlap(Sphere)
  (params (OverlappedComponent :type Primitive%20Component%20Object%20Reference) (OtherActor :type Actor%20Object%20Reference) (OtherComp :type Primitive%20Component%20Object%20Reference) (OtherBodyIndex :type Integer) (bFromSweep :type Boolean) (SweepResult :type Hit%20Result%20Structure%20%28by%20ref%29))
  (if (Actor|ActorHasTag OtherActor "Enemy")
    (Actor|DestroyActor OtherActor)
    (Niagara|SpawnSystematLocation "/Game/PiyoDash/Effects/FXS_Explosion.FXS_Explosion" (Transformation|GetActorLocation))))

(event EventBeginPlay
  (Transformation|SetWorldScale3D (Variables|Default|GetSphere) "0, 0, 0"))

(event Collision|EventActorBeginOverlap
  (params (OtherActor :type Actor%20Object%20Reference)))

(event EventTick
  (params (DeltaSeconds :type Float%20%28single-precision%29))
  (if (< (Variables|Default|GetScale) 4.0)
    (Variables|Default|SetScale (+ (Variables|Default|GetScale) (* 8.0 DeltaSeconds)))
    (Transformation|SetWorldScale3D (Variables|Default|GetSphere) (Math|Vector|MakeVector (Variables|Default|GetScale) (Variables|Default|GetScale) (Variables|Default|GetScale)))
    (else
      (Actor|DestroyActor))))

(fn ConstructionScript)